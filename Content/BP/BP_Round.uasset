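; Round manager actor that spawns enemies on a debug K key and drives their movement from a start point to an end point.
; CreateEnemy spawns the first EnemyConfig template at StartPos, initializes its path to EndPos, registers it in Enemies and loops a jog animation.
; Tick moves each enemy, destroying and removing those that cannot move, with hero damage only printed as a message.
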(event EventTick
  (params (DeltaSeconds :type Float%20%28single-precision%29))
  (if (> (Utilities|Array|Length (Variables|Default|GetEnemies)) 0)
    (for (_array_element _array_index) (Variables|Default|GetEnemies)
      (Utilities|IsValid _array_element
        (:Is%20Valid
          (if (Default|CouldMove _array_element)
            (Default|Move _array_element DeltaSeconds)
            (else
              (Actor|DestroyActor _array_element)
              (Utilities|Array|RemoveIndex (Variables|Default|GetEnemies) _array_index)
              (Development|PrintString "伤害结算：主角 HP -1"))))
        (:Is%20Not%20Valid
          (Development|PrintString "Not Valided" true true "(R=0.000000,G=0.660000,B=1.000000,A=1.000000)" 2.0 "MyTest"))))))

(event Input|KeyboardEvents|K
  (params (Key :type Key%20Structure :default "None"))
  (:Pressed
    (CallFunction|CreateEnemy)))

(fn ConstructionScript)

(fn CreateEnemy
  (bind _returnvalue (Game|SpawnActorfromClass (Utilities|Array|Get(acopy) (Variables|/Game/BP/BP_EnemyConfig.BP_EnemyConfig_C|GetEnemyTemplate (Variables|Default|GetEnemyConfig))) (Math|Transform|MakeTransform (Transformation|GetWorldLocation (Variables|Default|GetStartPos)) "0.000000,-90.000000,0.000000" "1.000000,1.000000,1.000000") "Undefined" "MultiplyWithRoot" 0 0))
  (Utilities|IsValid _returnvalue
    (:Is%20Valid
      (Utilities|FlowControl|Sequence
        (:then_0
          (Default|InitPos _returnvalue (Transformation|GetWorldLocation (Variables|Default|GetStartPos)) (Transformation|GetWorldLocation (Variables|Default|GetEndPos)))
          (Utilities|IsValid _returnvalue
            (:Is%20Valid
              (Utilities|Array|AddUnique (Variables|Default|GetEnemies) _returnvalue)
              (Components|Animation|PlayAnimation (Variables|/Script/Engine.Character|GetMesh _returnvalue) "/Game/Art/Characters/Mannequin_UE4/Animations/Jog_Fwd.Jog_Fwd" true)
              (return _returnvalue))))))))