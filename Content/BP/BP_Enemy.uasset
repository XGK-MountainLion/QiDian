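; BP_Enemy is an enemy that travels in a straight line from a start position toward an end position.
; InitPos stores both points and the normalized direction, and ResetPosToStart teleports the capsule back to the start.
; Move offsets the capsule by speed and delta time without sweeping, only while the mesh's world Y exceeds the end's Y.
; Tick is disabled and nothing here calls these functions.
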(event EventBeginPlay
  (|CallParentFunction))

(event Collision|EventActorBeginOverlap
  (params (OtherActor :type Actor%20Object%20Reference))
  (|CallParentFunction OtherActor) ; This node is disabled and will not be called.\nDrag off pins to build functionality.
)

(event EventTick
  (params (DeltaSeconds :type Float%20%28single-precision%29))
  (|CallParentFunction DeltaSeconds) ; This node is disabled and will not be called.\nDrag off pins to build functionality.
)

(fn ConstructionScript
  (|CallParentFunction))

(fn CouldMove
  (return (> (- (.y (Transformation|GetWorldLocation (Variables|Character|GetMesh))) (.y (Variables|Default|GetEndPos))) 0.0)))

(fn InitPos
  (params (StartPos :type Vector) (End :type Vector))
  (Utilities|FlowControl|Sequence
    (:then_0
      (bind _output_get (Variables|Default|SetStartPos StartPos)))
    (:then_1
      (bind _output_get_2 (Variables|Default|SetEndPos End)))
    (:then_2
      (Variables|Default|SetDirection (Math|Vector|Normalize (- _output_get_2 _output_get) 1.0)))))

(fn Move
  (params (deltaTime :type Float%20%28double-precision%29))
  (if (CallFunction|CouldMove)
    (Transformation|SetWorldLocation (Variables|Default|GetCapsuleComponent) (+ (Transformation|GetWorldLocation (Variables|Default|GetCapsuleComponent)) (* (Variables|Default|GetDirection) deltaTime (Variables|Default|GetMoveSpeed))) false false)))

(fn ResetPostoStart
  (Transformation|SetWorldLocation (Variables|Default|GetCapsuleComponent) (Variables|Default|GetStartPos) false false))